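; Example world-space task marker actor that shows a status icon through a StatusWidget_BP widget.
; On BeginPlay it turns once toward the player camera, then passes its icon to the widget and shows it after short delays.
; Each instance recounts all markers and sets every widget's color state from the clamped count or a disabled state, a shortcut the comments assign to a manager.
; ToggleTaskUI toggles icon visibility and destroys the actor when finished.
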(event Custom|ToggleTaskUI
  (params (bFinished :type Boolean) (bVisible :type Boolean))
  (Default|ToggleIcon (Variables|Default|GetMyStatusWidget) bVisible)
  (if bFinished
    (Actor|DestroyActor)))

(event EventBeginPlay
  ;[0 0 0] Pass along the icon, trigger the color
  (Utilities|FlowControl|Sequence
    (:then_0
      (Variables|Default|SetMyStatusWidget (.AsStatus%20Widget%20BP (Utilities|Casting|CastToStatusWidget_BP (UserInterface|GetUserWidgetObject (Variables|Default|GetWidget)))))
      (Utilities|FlowControl|Delay 0.1)
      (Transformation|SetActorRotation (Math|Rotator|FindLookatRotation (Transformation|GetActorLocation) (Camera|GetCameraLocation (Game|GetPlayerCameraManager 0)))))
    (:then_1
      ;[1 0 0 0.279] just to be super clear, this isn't how this should be done; a manager or the task itself should do this kind of thing
      (Utilities|FlowControl|Delay 0.2)
      (CallFunction|GetHowManyTasks)
      (Variables|/Game/OM_UI/StatusWidget_BP.StatusWidget_BP_C|SetCurrentStatusIcon (Variables|Default|GetMyStatusWidget) (Variables|Default|GetMyIcon))
      (Default|ToggleIcon (Variables|Default|GetMyStatusWidget) true))))

(fn ConstructionScript)

(fn GetHowManyTasks
  ;[1 0 0 0.47] This part would be handled by a manager, gamemode, etc, probably talking to the "taskl" that owns the widget. I.e., figure out what color we're supposed to be based on how many tasks are around
  (bind _outactors (Actor|GetAllActorsOfClass "ExampleUI_BP_C"))
  (bind _output_get (LocalVariables|Set_ExampleUIs _outactors))
  (LocalVariables|Set_numUIs (Utilities|Array|Length _output_get))
  (for _array_element (LocalVariables|Get_ExampleUIs)
    (Default|SetState (Variables|ExampleUI_BP_C|GetMyStatusWidget _array_element) (Utilities|Enum|ByteToEnumEStatusIconStates (select (Variables|ExampleUI_BP_C|GetbEnabled _array_element) (Math|Conversions|ToByte(Integer) (Math|Integer|Clamp(Integer) (- (LocalVariables|Get_numUIs) 1) 0 2)) 3)))))

(fn GetOurIcon)